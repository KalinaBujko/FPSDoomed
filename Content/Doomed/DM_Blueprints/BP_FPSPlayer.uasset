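; BP_FPSPlayer is a first-person player Blueprint that handles basic movement and mouse look.
; Horizontal and vertical axis inputs add movement along right and forward vectors taken from the control rotation's yaw only, so looking up or down does not affect direction.
; Mouse look axes feed controller yaw and pitch directly, and the construction script is empty.
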(event Input|AxisEvents|InputAxisHorizontalMovement
  (params (AxisValue :type Float%20%28single-precision%29))
  ;[0.9792 0.3764 0.6172 0.5] Movement
  (Pawn|Input|AddMovementInput (Math|Vector|GetRightVector (Math|Rotator|MakeRotator 0.0 0.0 (.yaw (Pawn|GetControlRotation :!class /Script/Engine.Pawn)))) AxisValue false))

(event Input|AxisEvents|InputAxisVerticalMovement
  (params (AxisValue :type Float%20%28single-precision%29))
  ;[0.9792 0.3764 0.6172 0.5] Movement
  (Pawn|Input|AddMovementInput (Math|Vector|GetForwardVector (Math|Rotator|MakeRotator 0.0 0.0 (.yaw (Pawn|GetControlRotation :!class /Script/Engine.Pawn)))) AxisValue false))

(event Input|AxisEvents|InputAxisMouseLookHorizontal
  (params (AxisValue :type Float%20%28single-precision%29))
  ;[0.402 0.1529 0.2542] Mouse Look
  (Pawn|Input|AddControllerYawInput AxisValue))

(event Input|AxisEvents|InputAxisMouseLookVertical
  (params (AxisValue :type Float%20%28single-precision%29))
  ;[0.402 0.1529 0.2542] Mouse Look
  (Pawn|Input|AddControllerPitchInput AxisValue))

(fn ConstructionScript)